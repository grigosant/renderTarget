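; BP_Player is the player for a canvas painting game, with mouse-look style yaw and pitch input and a HUD created on BeginPlay.
; Paint input line-traces from the camera and passes the hit UV, via FindCollisionUV, to BP_CanvasMy's ExecuteAction.
; Mode input repeats the trace and sets the hit canvas's EditMode from a player-side FlipFlop.
; An axis input adjusts a clamped BrushSize, which this Blueprint never passes to the canvas.
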(event EventBeginPlay
  (bind _returnvalue (UserInterface|CreateWidget "/Game/CanvasPainter/UI/WBP_HUD.WBP_HUD_C" 0 self))
  (UserInterface|Viewport|AddtoViewport _returnvalue 0))

(event Input|ActionEvents|InputActionPaintPoint
  (params (Key :type Key%20Structure :default "None"))
  (bind _returnvalue (Game|GetPlayerCameraManager 0))
  (bind _returnvalue_2 (Transformation|GetActorLocation _returnvalue))
  (:Pressed
    (bind _outhit (Collision|LineTraceByChannel _returnvalue_2 (+ _returnvalue_2 (* (Transformation|GetActorForwardVector _returnvalue) 1e+03)) "TraceTypeQuery1" true 0 "None"))
    (bind _asbp_canvas_my (Utilities|Casting|CastToBP_CanvasMy (.HitActor (Collision|BreakHitResult _outhit))))
    (Default|ExecuteAction _asbp_canvas_my (.UV (Class|GameplayStatics|FindCollisionUV _outhit)))))

(event Input|ActionEvents|InputActionChangeMode
  (params (Key :type Key%20Structure :default "None"))
  (bind _returnvalue (Game|GetPlayerCameraManager 0))
  (bind _returnvalue_2 (Transformation|GetActorLocation _returnvalue))
  (:Pressed
    (bind _outhit (Collision|LineTraceByChannel _returnvalue_2 (+ _returnvalue_2 (* (Transformation|GetActorForwardVector _returnvalue) 1e+03)) "TraceTypeQuery1" true 0 "None"))
    (bind _asbp_canvas_my (Utilities|Casting|CastToBP_CanvasMy (.HitActor (Collision|BreakHitResult _outhit))))
    (bind _isa (Utilities|FlowControl|FlipFlop)
      (:A
        _)
      (:B
        _))
    (Variables|/Game/CanvasPainter/Blueprints/BP_CanvasMy.BP_CanvasMy_C|SetbEditMode _asbp_canvas_my _isa)))

(event Input|AxisEvents|InputAxisLookRight
  (params (AxisValue :type Float%20%28single-precision%29))
  (Pawn|Input|AddControllerYawInput AxisValue))

(event Input|AxisEvents|InputAxisLookUp
  (params (AxisValue :type Float%20%28single-precision%29))
  (Pawn|Input|AddControllerPitchInput AxisValue))

(event Input|AxisEvents|InputAxisChangeBrushSize
  (params (AxisValue :type Float%20%28single-precision%29))
  (Variables|Default|SetBrushSize (Math|Float|Clamp(Float) (+ (* AxisValue 1e+01) (Variables|Default|GetBrushSize)) 0.0 1e+03)))

(fn ConstructionScript)