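; Paintable canvas actor that lets polygon regions be outlined on an image and later identified by point.
; BeginPlay draws the background into a render target shown on the Canvas through a dynamic material.
; In EditMode, executeAction adds points outside existing figures, drawing lines until one lands near the first, then stores the figure and calls CallFinish.
; Otherwise it prints the description of the figure hit, using an even-odd ray-crossing test.
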(event Custom|executeAction
  (params (PointLocation :type Vector%202D%20Structure))
  (if (Variables|Default|GetbEditMode)
    (bind _success (CallFunction|CheckPointAllFigures PointLocation))
    (if (not _success)
      (CallFunction|AddPoint PointLocation))
    (else
      (bind (_success_2 _array_index) (CallFunction|CheckPointAllFigures PointLocation))
      (if _success_2
        (bind _output_get (Variables|Default|SetFigureName (.figuredescription (Utilities|Array|Get(acopy) (Variables|Default|GetAllFigures) _array_index))))
        (Development|PrintString _output_get true true "(R=0.000000,G=0.660000,B=1.000000,A=1.000000)" 5.0)
        (else
          (Development|PrintString "Не попал" true true "(R=0.000000,G=0.660000,B=1.000000,A=1.000000)" 5.0))))))

(event Custom|changeMode
  (bind _result (Math|Integer|IncrementInt (Variables|Default|GetcurrentMode))
    (:%20%20
      (Variables|Default|SetcurrentMode (Math|Integer|%(Integer) _result 2)))))

(event EventBeginPlay
  (Utilities|FlowControl|Sequence
    (:then_0
      (bind _returnvalue (Rendering|CreateRenderTarget2D 2048 4096 "RTF_RGBA16f"))
      (bind _output_get (Variables|Default|SetTarget _returnvalue))
      (bind (_canvas _size _context) (Rendering|BeginDrawCanvastoRenderTarget (Variables|Default|GetTarget)))
      (Canvas|DrawTexture :self _canvas :RenderTexture (Variables|Default|GetbackgroundImage) :ScreenSize _size :CoordinateSize "(X=1.000000,Y=1.000000)" :BlendMode "BLEND_Opaque" :PivotPoint "(X=0.500000,Y=0.500000)")
      (Rendering|EndDrawCanvastoRenderTarget _context))
    (:then_1
      (bind _returnvalue_2 (Rendering|Material|CreateDynamicMaterialInstance "/Game/CanvasPainter/Materials/M_Canvas.M_Canvas" "None" "None" :!class /Script/Engine.KismetMaterialLibrary))
      (Rendering|Material|SetTextureParameterValue _returnvalue_2 "RenderTarget" (Variables|Default|GetTarget))
      (Rendering|Material|SetMaterial (Variables|Default|GetCanvas) 0 _returnvalue_2))
    (:then_2
      (bind _returnvalue_3 (Rendering|Material|CreateDynamicMaterialInstance "/Game/CanvasPainter/Materials/M_Brush.M_Brush" "None" "None" :!class /Script/Engine.KismetMaterialLibrary))
      (Variables|Brush|SetBrushMaterial _returnvalue_3))))

(fn ConstructionScript)

(fn DrawBrush
  (params (DrawLocation :type Vector%202D%20Structure))
  (bind _brushsize (Variables|Brush|GetBrushSize))
  (Utilities|FlowControl|Sequence
    (:then_0
      (Rendering|Material|SetTextureParameterValue (Variables|Brush|GetBrushMaterial) "BrushTexture" (Variables|Brush|GetBrushTexture)))
    (:then_1
      (bind (_canvas _size _context) (Rendering|BeginDrawCanvastoRenderTarget (Variables|Default|GetTarget)))
      (Canvas|DrawTexture :self _canvas :RenderTexture (Variables|Brush|GetBrushTexture) :ScreenPosition (- (* _size DrawLocation) (/ (Variables|Brush|GetBrushSize) 2.0)) :ScreenSize (Math|Vector2D|MakeVector2D _brushsize _brushsize) :CoordinateSize "(X=1.000000,Y=1.000000)" :PivotPoint "(X=0.500000,Y=0.500000)")
      (Rendering|EndDrawCanvastoRenderTarget _context))))

(fn AddPoint
  (params (DrawLocation :type Vector%202D%20Structure))
  (if (Variables|Default|GetarePointsExist)
    (bind _needtofinish (CallFunction|CheckFinishFigure DrawLocation))
    (if _needtofinish
      (CallFunction|FinishFigure)
      (Development|PrintString "figure finished" true true "(R=0.000000,G=0.660000,B=1.000000,A=1.000000)" 5.0)
      (else
        (CallFunction|DrawLine DrawLocation)
        (Utilities|Array|Add (Variables|Default|GetcurrentFigure) DrawLocation)))
    (else
      (Utilities|Array|Add (Variables|Default|GetcurrentFigure) DrawLocation)
      (Variables|Default|SetarePointsExist true))))

(fn DrawLine
  (params (DrawLocation :type Vector%202D%20Structure))
  (bind _currentfigure (Variables|Default|GetcurrentFigure))
  (bind (_canvas _size _context) (Rendering|BeginDrawCanvastoRenderTarget (Variables|Default|GetTarget)))
  (Class|Canvas|DrawLine _canvas (* _size (Utilities|Array|Get(acopy) _currentfigure (- (Utilities|Array|Length _currentfigure) 1))) (* _size DrawLocation) 3.0 (Variables|Default|GetLineColor))
  (Rendering|EndDrawCanvastoRenderTarget _context))

(fn CheckFinishFigure
  (params (NewPoint :type Vector%202D%20Structure))
  (if (> (Utilities|Array|Length (Variables|Default|GetcurrentFigure)) 1)
    (if (> (Variables|Default|Getepsilon) (Math|Vector|Distance2D(Vector) NewPoint (Utilities|Array|Get(acopy) (Variables|Default|GetcurrentFigure))))
      (return true)
      (else
        _)))
  (return false))

(fn FinishFigure
  (CallFunction|DrawLine (Utilities|Array|Get(acopy) (Variables|Default|GetcurrentFigure)))
  (Utilities|Array|Add (Variables|Default|GetAllFigures) (Utilities|Struct|MakeS_Figure (Variables|Default|GetcurrentFigure) (Utilities|String|Append "Выбрана область №" (Utilities|String|ToString(Integer) (+ (Utilities|Array|Length (Variables|Default|GetAllFigures)) 1)))))
  (Utilities|Array|Clear (Variables|Default|GetcurrentFigure))
  (Variables|Default|SetarePointsExist false)
  (Default|CallFinish))

(fn CheckPointIntoFigure
  (params (Point :type Vector%202D%20Structure) (figure :type Array%20of%20Vector%202D%20Structures))
  (if true
    (LocalVariables|SetPreviousPoint (Utilities|Array|Get(acopy) figure (Utilities|Array|LastIndex figure)))
    (for _array_element figure
      (LocalVariables|SetcurrentPoint _array_element)
      (if (and (or (and (< (.y (LocalVariables|GetcurrentPoint)) (.y Point)) (>= (.y (LocalVariables|GetPreviousPoint)) (.y Point))) (and (>= (.y (LocalVariables|GetcurrentPoint)) (.y Point)) (< (.y (LocalVariables|GetPreviousPoint)) (.y Point)))) (< (+ (.x (LocalVariables|GetcurrentPoint)) (* (- (.x (LocalVariables|GetPreviousPoint)) (.x (LocalVariables|GetcurrentPoint))) (/ (- (.y Point) (.y (LocalVariables|GetcurrentPoint))) (- (.y (LocalVariables|GetPreviousPoint)) (.y (LocalVariables|GetcurrentPoint)))))) (.x Point)))
        (LocalVariables|Setresult (not (LocalVariables|Getresult))))
      (LocalVariables|SetPreviousPoint (LocalVariables|GetcurrentPoint)))
    (return (LocalVariables|Getresult))))

(fn CheckPointAllFigures
  (params (Point :type Vector%202D%20Structure))
  (for (_array_element _array_index) (Variables|Default|GetAllFigures)
    (bind _resultvalue (CallFunction|CheckPointIntoFigure Point (.figurespoints (Utilities|Struct|BreakS_Figure _array_element))))
    (if _resultvalue
      (return true _array_index)))
  (return false 0))