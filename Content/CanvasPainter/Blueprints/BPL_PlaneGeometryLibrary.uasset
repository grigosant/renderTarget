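; Blueprint function library of 2D plane geometry helpers in CanvasPainter.
; Lines are slope-intercept vectors (X slope, Y intercept), built from two points or a point and direction, and circles pack center and radius.
; It finds line-line and line-circle intersections, the latter through a quadratic solver that reports root count.
; Vertical lines are unsupported, and only the normal-line function checks for a zero divisor.
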(fn Lineby2Points
  (params (point1 :type Vector%202D%20Structure) (point2 :type Vector%202D%20Structure))
  (LocalVariables|Setx1 (.x point1))
  (LocalVariables|Sety1 (.y point1))
  (LocalVariables|Setx2 (.x point2))
  (LocalVariables|Sety2 (.y point2))
  (return (Math|Vector2D|MakeVector2D (/ (- (LocalVariables|Gety2) (LocalVariables|Gety1)) (- (LocalVariables|Getx2) (LocalVariables|Getx1))) (/ (- (* (LocalVariables|Getx2) (LocalVariables|Gety1)) (* (LocalVariables|Getx1) (LocalVariables|Gety2))) (- (LocalVariables|Getx2) (LocalVariables|Getx1))))))

(fn NormalLineThroughtPoint
  (params (point :type Vector%202D%20Structure) (normal :type Vector%202D%20Structure))
  (LocalVariables|Setx0 (.x point))
  (LocalVariables|Sety0 (.y point))
  (LocalVariables|Setp1 (.x normal))
  (LocalVariables|Setp2 (.y normal))
  (if (!= (LocalVariables|Getp1) 0.0)
    (return (Math|Vector2D|MakeVector2D (/ (LocalVariables|Getp2) (LocalVariables|Getp1)) (- (LocalVariables|Gety0) (* (/ (LocalVariables|Getp2) (LocalVariables|Getp1)) (LocalVariables|Getx0)))))))

(fn PointOf2LineCrossing
  (params (line%201 :type Vector%202D%20Structure) (line%202 :type Vector%202D%20Structure))
  (bind _returnvalue (- (.y line%202) (.y line%201)))
  (bind _returnvalue_2 (- (.x line%201) (.x line%202)))
  (bind _returnvalue_3 (/ _returnvalue _returnvalue_2))
  (return (Math|Vector2D|MakeVector2D _returnvalue_3 (+ (* (.x line%201) _returnvalue_3) (.y line%201)))))

(fn PointOfCircleandLine
  (params (Circle :type Vector) (Line :type Vector%202D%20Structure))
  (LocalVariables|Setx0 (.x Circle))
  (LocalVariables|Sety0 (.y Circle))
  (LocalVariables|Setr (.z Circle))
  (LocalVariables|Setk (.x Line))
  (LocalVariables|Setb (.y Line))
  (bind (_numofroots _firstroot _secondroot) (CallFunction|QuadraticEquation (Math|Vector|MakeVector (+ (* (LocalVariables|Getk) (LocalVariables|Getk)) 1.0) (- (- (* 2.0 (LocalVariables|Getk) (LocalVariables|Getb)) (* 2.0 (LocalVariables|Getx0))) (* 2.0 (LocalVariables|Getk) (LocalVariables|Gety0))) (- (- (+ (* (LocalVariables|Getx0) (LocalVariables|Getx0)) (* (LocalVariables|Gety0) (LocalVariables|Gety0)) (* (LocalVariables|Getb) (LocalVariables|Getb))) (* 2.0 (LocalVariables|Getb) (LocalVariables|Gety0))) (* (LocalVariables|Getr) (LocalVariables|Getr))))))
  (return _numofroots (Math|Vector2D|MakeVector2D _firstroot (+ (* (LocalVariables|Getk) _firstroot) (LocalVariables|Getb))) (Math|Vector2D|MakeVector2D _secondroot (+ (* (LocalVariables|Getk) _secondroot) (LocalVariables|Getb)))))

(fn QuadraticEquation
  (params (koefficiets :type Vector))
  (LocalVariables|Seta (.x koefficiets))
  (LocalVariables|Setb (.y koefficiets))
  (LocalVariables|Setc (.z koefficiets))
  (bind _output_get (LocalVariables|SetDiskriminant (- (* (LocalVariables|Getb) (LocalVariables|Getb)) (* 4.0 (LocalVariables|Geta) (LocalVariables|Getc)))))
  (if (< _output_get 0.0)
    (return 0 0.0 0.0) ; корней нет
    (elif (== (LocalVariables|GetDiskriminant) 0.0)
      (return 1 (/ (* -1.0 (LocalVariables|Getb)) (* (LocalVariables|Geta) 2.0)) 0.0) ; 1 корень
      (else
        (return 2 (/ (+ (* -1.0 (LocalVariables|Getb)) (Math|Float|Sqrt (LocalVariables|GetDiskriminant))) (* (LocalVariables|Geta) 2.0)) (/ (- (* -1.0 (LocalVariables|Getb)) (Math|Float|Sqrt (LocalVariables|GetDiskriminant))) (* (LocalVariables|Geta) 2.0))) ; 2 корня
      ))))